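; BP_Projectile is a short-lived projectile actor whose speed builds on the player's current speed.
; When its ProjectileMovement component activates, it casts player pawn 0 to BP_Player and sets initial and max speed to UpdatedSpeed plus a fixed offset.
; Tick accumulates elapsed time and destroys the actor after two seconds.
; The overlap and sphere hit events are empty, so this graph handles no impacts.
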(event OnComponentHit(Sphere)
  (params (HitComponent :type Primitive%20Component%20Object%20Reference) (OtherActor :type Actor%20Object%20Reference) (OtherComp :type Primitive%20Component%20Object%20Reference) (NormalImpulse :type Vector :default "0, 0, 0") (Hit :type Hit%20Result%20Structure%20%28by%20ref%29)))

(event OnComponentActivated(ProjectileMovement)
  (params (Component :type Actor%20Component%20Object%20Reference) (bReset :type Boolean))
  (bind _projectilemovement (Variables|Default|GetProjectileMovement))
  (bind _asbp_player (Utilities|Casting|CastToBP_Player (Game|Player|GetPlayerPawn 0)))
  (Variables|/Script/Engine.ProjectileMovementComponent|SetInitialSpeed _projectilemovement (+ (Variables|/Game/InfiniteMatrix/Blueprints/BP_Player.BP_Player_C|GetUpdatedSpeed _asbp_player) 2e+03))
  (Variables|/Script/Engine.ProjectileMovementComponent|SetMaxSpeed _projectilemovement (+ (Variables|/Game/InfiniteMatrix/Blueprints/BP_Player.BP_Player_C|GetUpdatedSpeed _asbp_player) 2e+03)))

(event Collision|EventActorBeginOverlap
  (params (OtherActor :type Actor%20Object%20Reference)))

(event EventTick
  (params (DeltaSeconds :type Float%20%28single-precision%29))
  (bind _output_get (Variables|Default|SetTimeOfExistence (+ DeltaSeconds (Variables|Default|GetTimeOfExistence))))
  (if (>= _output_get 2.0)
    (Actor|DestroyActor)))

(fn ConstructionScript)